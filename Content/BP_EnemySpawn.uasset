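; Spawner actor that periodically creates BP_Enemy instances at random points inside its SpawnZone box while a player character exists.
; If IsActive is set at BeginPlay, it starts a looping timer with a random delay whose upper limit shrinks as real time elapses.
; Each successful spawn gives the enemy its default controller, then re-sets the timer with a newly randomized delay, so spawning tends to speed up over time.
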(event Custom|SpawnTimer
  (bind _spawnzone (Variables|Default|GetSpawnZone))
  (bind _spawntime (Variables|Default|GetSpawnTime))
  (bind _returnvalue (Components|Box|GetScaledBoxExtent _spawnzone))
  (bind _returnvalue_2 (Transformation|GetWorldLocation _spawnzone))
  (bind _returnvalue_3 (Math|Random|RandomPointinBoundingBox _returnvalue_2 _returnvalue))
  (if (Utilities|IsValid (Game|GetPlayerCharacter 0))
    (bind _returnvalue_4 (Game|SpawnActorfromClass "/Game/BP_Enemy.BP_Enemy_C" (Math|Transform|MakeTransform (Math|Vector|MakeVector (.x _returnvalue_3) (.y _returnvalue_3) (.z _returnvalue_3)) "0, 0, 0" "1.000000,1.000000,1.000000") "Undefined" "MultiplyWithRoot" 0 0))
    (if (Utilities|IsValid _returnvalue_4)
      (Pawn|SpawnDefaultController _returnvalue_4)
      (Utilities|Time|SetTimerbyEvent (delegate Custom|SpawnTimer) (Math|Random|RandomFloatinRange 0.0 (+ (- _spawntime (/ (/ (Utilities|Time|GetRealTimeSeconds) _spawntime) 1e+01)) (/ 0.0 2.0))) true))))

(event EventBeginPlay
  (bind _spawntime (Variables|Default|GetSpawnTime))
  (if (Variables|Default|GetIsActive)
    (Utilities|Time|SetTimerbyEvent (delegate Custom|SpawnTimer) (Math|Random|RandomFloatinRange 0.0 (+ (- _spawntime (/ (/ (Utilities|Time|GetRealTimeSeconds) _spawntime) 1e+01)) (/ 0.0 2.0))) true)))

(fn ConstructionScript)