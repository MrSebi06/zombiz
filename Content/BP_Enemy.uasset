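; BP_Enemy is an enemy that chases the player and attacks within range.
; Tick steers it straight at the player with movement input and rotation, without pathfinding, and calls a cooldown-gated Attack when close enough.
; An enum-guarded ChangeState plays idle, walk or attack animations directly on the mesh, only on state changes.
; TakeDamage reduces HP and, at zero or below, destroys the enemy and adds the final hit's damage to the player's score.
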(event EventTick
  (params (DeltaSeconds :type Float%20%28single-precision%29))
  (bind _returnvalue (Transformation|GetActorLocation))
  (bind _returnvalue_2 (Game|GetPlayerCharacter 0))
  (bind _returnvalue_3 (Transformation|GetActorLocation _returnvalue_2))
  (bind _returnvalue_4 (Math|Vector|GetUnitDirection(Vector) _returnvalue _returnvalue_3))
  (if (Utilities|IsValid _returnvalue_2)
    ;[0.8754 1 0.7906] Move Towards Player
    (if (<= (Math|Vector|VectorLength (- _returnvalue _returnvalue_3)) (Variables|Default|GetRange))
      (bind _asbp_first_person_character (Utilities|Casting|CastToBP_FirstPersonCharacter _returnvalue_2))
      (CallFunction|Attack _asbp_first_person_character)
      (else
        (CallFunction|ChangeState "NewEnumerator1")
        (Pawn|Input|AddMovementInput _returnvalue_4 (Variables|Default|GetSpeed) false)
        (Transformation|SetActorRotation (Math|Conversions|RotationFromXVector _returnvalue_4))))
    (else
      (CallFunction|ChangeState "NewEnumerator0"))))

(event EventBeginPlay
  (Components|Animation|PlayAnimation (Variables|Character|GetMesh) "/Game/External/BookHeadMonster/Demo/Animations/MM_Walk_Fwd.MM_Walk_Fwd" true))

(fn ConstructionScript)

(fn TakeDamage
  (params (Damage :type Float%20%28double-precision%29))
  (bind _output_get (Variables|Default|SetHP (- (Variables|Default|GetHP) Damage)))
  (Math|Float|CompareFloat _output_get 0.0
    (:==
      _)
    (:<
      _))
  (Actor|DestroyActor)
  (bind _asbp_first_person_character (Utilities|Casting|CastToBP_FirstPersonCharacter (Game|Player|GetPlayerPawn 0)))
  (Default|AddScore _asbp_first_person_character (Math|Conversions|ToInteger(Byte) (Class|KismetMathLibrary|ToInt64(Float) Damage))))

(fn Attack
  (params (Player :type BP%20First%20Person%20Character%20Object%20Reference))
  (bind _returnvalue (Utilities|Time|GetRealTimeSeconds))
  (if (>= (- _returnvalue (Variables|Default|GetLastAttackTime)) (Variables|Default|GetAttackCoolDown))
    (CallFunction|ChangeState "NewEnumerator2")
    (Default|TakeDamage Player (Variables|Default|GetAttackDamage))
    (Variables|Default|SetLastAttackTime _returnvalue)
    (elif (> (- _returnvalue (Variables|Default|GetLastAttackTime)) 0.6)
      (CallFunction|ChangeState "NewEnumerator0"))))

(fn ChangeState
  (params (NewState :type EnemyStateEnum%20Enum :default "NewEnumerator0"))
  (if (not (Utilities|Enum|Equal(Enum) NewState (Variables|Default|GetState)))
    (switch Utilities|FlowControl|Switch|SwitchonEnemyStateEnum NewState
      (:NewEnumerator0
        (Components|Animation|PlayAnimation (Variables|Character|GetMesh) "/Game/External/BookHeadMonster/Demo/Animations/MM_Idle.MM_Idle" true)
        (Variables|Default|SetState "NewEnumerator0"))
      (:NewEnumerator1
        (Components|Animation|PlayAnimation (Variables|Character|GetMesh) "/Game/External/BookHeadMonster/Demo/Animations/MM_Walk_InPlace.MM_Walk_InPlace" true)
        (Variables|Default|SetState "NewEnumerator1"))
      (:NewEnumerator2
        (Components|Animation|PlayAnimation (Variables|Character|GetMesh) "/Game/External/BookHeadMonster/Demo/Animations/MM_Land.MM_Land" false)
        (Variables|Default|SetState "NewEnumerator2")))))